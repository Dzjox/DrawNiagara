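; Player controller for a cursor-driven drawing scene that routes Enhanced Input actions to a BP_DrawManager.
; On BeginPlay it finds the draw sphere and manager, gives the manager the sphere to follow, and sets its grid location from the "Canvas"-tagged actor.
; Each tick the sphere sweeps to the cursor's trace hit point.
; Input triggers drawing, erasing, render target switching, and clearing of the canvas and both sand-map render targets.
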(event `self.ReceiveBeginPlay`
  (`|ExecutionSequence`
    (:`then_0`
      (`EnhancedInputSubsystemInterface.AddMappingContext` (subsystem `EnhancedInputLocalPlayerSubsystem`) "/Game/DrawNiagara/Input/IMC_Main.IMC_Main" 0 (struct)))
    (:`then_1`
      (bind _returnvalue (`GameplayStatics.GetActorOfClass` "/Game/DrawNiagara/Blueprints/BP_DrawSphere.BP_DrawSphere_C"))
      (set `self.DrawSphere` _returnvalue))
    (:`then_3`
      (bind _returnvalue_2 (`GameplayStatics.GetActorOfClass` "/Game/DrawNiagara/Blueprints/BP_DrawManager.BP_DrawManager_C"))
      (bind _output_get (set `self.DrawManager` _returnvalue_2))
      (`DrawManager.SetSphereComponentsToFollow` _output_get (`|MakeArray` (`/Game/DrawNiagara/Blueprints/BP_DrawSphere.Sphere` (`self.DrawSphere`))))
      (`DrawManager.NewStart` _output_get))
    (:`then_4`
      (bind _outactors (`GameplayStatics.GetAllActorsWithTag` "Canvas"))
      (`DrawManager.SetGridLocation` (`self.DrawManager`) (`self.K2_GetActorLocation` (`|GetArrayItem` _outactors))))))

(event `self.ReceiveTick`
  (params (DeltaSeconds :type "Float (single-precision)"))
  (`self.K2_SetActorLocation` (`self.DrawSphere`) (`.Location` (`GameplayStatics.BreakHitResult` (`self.GetHitResultUnderCursorByChannel` "TraceTypeQuery1"))) true true))

(event `EnhancedInput|/Game/DrawNiagara/Input/IA_ScreenTouch`
  (params (ActionValue :type Boolean) (ElapsedSeconds :type "Float (double-precision)") (TriggeredSeconds :type "Float (double-precision)") (InputAction :type "InputAction Object Reference" :default "/Game/DrawNiagara/Input/IA_ScreenTouch.IA_ScreenTouch"))
  (:`Triggered`
    (`DrawManager.Draw` (`self.DrawManager`))))

(event `EnhancedInput|/Game/DrawNiagara/Input/IA_ClearScreen`
  (params (ActionValue :type Boolean) (ElapsedSeconds :type "Float (double-precision)") (TriggeredSeconds :type "Float (double-precision)") (InputAction :type "InputAction Object Reference" :default "/Game/DrawNiagara/Input/IA_ClearScreen.IA_ClearScreen"))
  (:`Started`
    (`DrawManager.ClearCanvas` (`self.DrawManager`))
    (`KismetRenderingLibrary.ClearRenderTarget2D` "/Game/DrawNiagara/RTs/RT_SandMap.RT_SandMap")
    (`KismetRenderingLibrary.ClearRenderTarget2D` "/Game/DrawNiagara/RTs/RT_SandMap_Extra.RT_SandMap_Extra")))

(event `EnhancedInput|/Game/DrawNiagara/Input/IA_Eraser`
  (params (ActionValue :type Boolean) (ElapsedSeconds :type "Float (double-precision)") (TriggeredSeconds :type "Float (double-precision)") (InputAction :type "InputAction Object Reference" :default "/Game/DrawNiagara/Input/IA_Eraser.IA_Eraser"))
  (:`Triggered`
    (`DrawManager.Erase` (`self.DrawManager`))))

(event `EnhancedInput|/Game/DrawNiagara/Input/IA_ChangeRenderTarget`
  (params (ActionValue :type Boolean) (ElapsedSeconds :type "Float (double-precision)") (TriggeredSeconds :type "Float (double-precision)") (InputAction :type "InputAction Object Reference" :default "/Game/DrawNiagara/Input/IA_ChangeRenderTarget.IA_ChangeRenderTarget"))
  (:`Started`
    (`DrawManager.SwitchRT` (`self.DrawManager`))
    (`KismetSystemLibrary.PrintString` "Hello")))

(fn `UserConstructionScript`)