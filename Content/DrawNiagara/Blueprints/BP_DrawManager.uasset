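; Manager Blueprint for a Niagara-based drawing system that paints or erases along the paths of tracked sphere components.
; It interpolates evenly spaced points between each sphere's previous and current location, avoiding gaps in fast strokes.
; Points packed with radius, plus stroke directions, go to the Niagara solver through array parameters, then get cleared.
; A macro toggles the solver's eraser flag, and clearing pulses a canvas flag across a zero-length delay.
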(event `ResetNiagara`
  (`NiagaraComponent.ResetSystem` (`self.NS_DrawSolver`)))

(event `SetSphereComponentsToFolow`
  (params (DrawingSpheres :type "Array of SphereComponent Object Reference"))
  (set `self.DrawingSpheres` DrawingSpheres)
  (`KismetArrayLibrary.Array_Clear` (`self.DrawingPositionsAndRadius`))
  (`KismetArrayLibrary.Array_Clear` (`self.DrawingDirections`))
  (`KismetArrayLibrary.Array_Resize` (`self.PrevLocation`) (`KismetArrayLibrary.Array_Length` (`self.DrawingSpheres`))))

(event `NewStart`
  (`KismetArrayLibrary.Array_Clear` (`self.PrevLocation`))
  (`KismetArrayLibrary.Array_Resize` (`self.PrevLocation`) (`KismetArrayLibrary.Array_Length` (`self.DrawingSpheres`)))
  (for (_array_element _array_index) (`self.DrawingSpheres`)
    (`KismetArrayLibrary.Array_Set` (`self.PrevLocation`) _array_index (`SceneComponent.K2_GetComponentLocation` _array_element))))

(event `Draw`
  (`self.SwitchModDrawErase` :!label _label
    (:`Exec`
      (`|ExecutionSequence`
        (:`then_0`
          (for (_array_element _array_index) (`self.DrawingSpheres`)
            (set `self.CurrentSphere` _array_element)
            (bind _output_get (set `self.SphereIndex` _array_index))
            (if (== (`|GetArrayItem` (`self.PrevLocation`) _output_get) (0.0 0.0 0.0) :`ErrorTolerance` 0.1)
              ;[1 1 1] Do not draw if have no info about prev location
              (`KismetArrayLibrary.Array_Set` (`self.PrevLocation`) (`self.SphereIndex`) (`SceneComponent.K2_GetComponentLocation` (`self.CurrentSphere`)))
              (elif (`self.WasMovement`)
                (bind (_points _normal) (`self.FindPointsBettwenLocationsWithDistance` (`SceneComponent.K2_GetComponentLocation` (`self.CurrentSphere`)) (`|GetArrayItem` (`self.PrevLocation`) (`self.SphereIndex`)) (`self.DistanceВetweenDraws`)))
                (for _array_element_2 _points
                  (`KismetArrayLibrary.Array_Add` (`self.DrawingPositionsAndRadius`) (`KismetMathLibrary.MakeVector4` (.x _array_element_2) (.y _array_element_2) (.z _array_element_2) (`SphereComponent.SphereRadius` (`self.CurrentSphere`))))
                  (`KismetArrayLibrary.Array_Add` (`self.DrawingDirections`) _normal))
                (`KismetArrayLibrary.Array_Set` (`self.PrevLocation`) (`self.SphereIndex`) (`SceneComponent.K2_GetComponentLocation` (`self.CurrentSphere`)))))))
        (:`then_1`
          ;[1 1 1] Send location, radius and direction data to Niagara solver
          (`NiagaraDataInterfaceArrayFunctionLibrary.SetNiagaraArrayVector4` (`self.NS_DrawSolver`) "DrawingLocationsAndRadiuses" (`self.DrawingPositionsAndRadius`))
          (`NiagaraDataInterfaceArrayFunctionLibrary.SetNiagaraArrayVector` (`self.NS_DrawSolver`) "DrawingDirections" (`self.DrawingDirections`))
          ;[1 0 0] Можно сетать один раз в самом начале
          (`NiagaraComponent.SetVariableVec3` (`self.NS_DrawSolver`) "GridLocation" (`self.GridLocation`))
          (`NiagaraComponent.SetVariableFloat` (`self.NS_DrawSolver`) "EraseStrenght" (`self.EraseStrenght`))
          (`KismetArrayLibrary.Array_Clear` (`self.DrawingPositionsAndRadius`))
          (`KismetArrayLibrary.Array_Clear` (`self.DrawingDirections`)))))))

(event `Erase`
  (goto _label :!via `Erase`))

(event `ClearScreen`
  (`NiagaraComponent.SetVariableBool` (`self.NS_DrawSolver`) "ClearCanvas" true)
  (`NiagaraDataInterfaceArrayFunctionLibrary.SetNiagaraArrayVector4` (`self.NS_DrawSolver`) "DrawingLocationsAndRadiuses" (`|MakeArray`))
  (`NiagaraDataInterfaceArrayFunctionLibrary.SetNiagaraArrayVector` (`self.NS_DrawSolver`) "DrawingDirections" (`|MakeArray`))
  ;[1 1 1] Time for niagara processed input
  (`KismetSystemLibrary.Delay` 0.0)
  (`NiagaraComponent.SetVariableBool` (`self.NS_DrawSolver`) "ClearCanvas" false)
  (`KismetArrayLibrary.Array_Clear` (`self.PrevLocation`))
  (`KismetArrayLibrary.Array_Resize` (`self.PrevLocation`) (`KismetArrayLibrary.Array_Length` (`self.DrawingSpheres`))))

(fn `FindPointsBettwenLocationsWithDistance`
  (params (End :type "Vector Structure") (Start :type "Vector Structure") (DistanceBettwen :type "Float (double-precision)"))
  (returns (Points :type "Array of Vector Structure") (Normal :type "Vector Structure"))
  (locals (Length :type "Float (double-precision)" :default 0.0) (IterationsCount :type Integer :default 0) (Result :type "Array of Vector Structure") (NormalazedVector :type "Vector Structure" :default (0.0 0.0 0.0)))
  (bind _returnvalue (- End Start))
  (bind _result (`local.Result`))
  (bind _output_get (set `local.Length` (`KismetMathLibrary.VSize` _returnvalue)))
  (bind _output_get_2 (set `local.IterationsCount` (`KismetMathLibrary.FFloor` (/ _output_get DistanceBettwen))))
  (bind _output_get_3 (set `local.NormalazedVector` (`KismetMathLibrary.MakeVector` (/ (.x _returnvalue) _output_get) (/ (.y _returnvalue) _output_get) (/ (.z _returnvalue) _output_get))))
  (for _index (range (+ _output_get_2 1))
    (`KismetArrayLibrary.Array_Add` _result (+ Start (* _index _output_get_3 DistanceBettwen))))
  (return _result _output_get_3))

(fn `UserConstructionScript`)

(fn `WasMovement`
  (returns (ReturnValue :type Boolean))
  (return (> (`KismetMathLibrary.VSizeSquared` (- (`SceneComponent.K2_GetComponentLocation` (`self.CurrentSphere`)) (`|GetArrayItem` (`self.PrevLocation`) (`self.SphereIndex`)))) 0.1)))