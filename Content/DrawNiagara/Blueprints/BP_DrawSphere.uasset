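; BP_DrawSphere is a placeable sphere actor that registers itself as a drawing sphere with the level's BP_DrawManager.
; Its Construction Script applies Radius and HiddenInGame to the Sphere component, then finds the manager by the "DrawManager" actor tag.
; It adds itself to DrawingSpheres unless an entry has the same object name, and prints red errors for a missing, duplicate or wrongly tagged manager.
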(fn `UserConstructionScript`
  (`|ExecutionSequence`
    (:`then_0`
      ;[1 1 1] Set default properties
      (`SphereComponent.SetSphereRadius` (`self.Sphere`) (`self.Radius`) true)
      (`SceneComponent.SetHiddenInGame` (`self.Sphere`) (`self.HiddenInGame`) false))
    (:`then_1`
      ;[1 1 1] Checks for errors
      (bind _outactors (`GameplayStatics.GetAllActorsWithTag` "DrawManager"))
      (bind _returnvalue (`KismetArrayLibrary.Array_Length` _outactors))
      (if (== _returnvalue 0)
        (`KismetSystemLibrary.PrintString` "ERROR! DrawManager doesn`t exist!" true true (struct :`R` 1.0 :`A` 1.0) 5.0 "DrawSphere")
        (elif (== _returnvalue 1)
          (bind _asbp_draw_manager (cast `/Game/DrawNiagara/Blueprints/BP_DrawManager` (`|GetArrayItem` _outactors))
            (:`then`
              ;[1 1 1] Add self as draw sphere to draw manager
              (if (not (`self.bHasSelfInManager`))
                (bind _drawingspheres (`/Game/DrawNiagara/Blueprints/BP_DrawManager.DrawingSpheres` _asbp_draw_manager))
                (for _array_element _drawingspheres
                  ;;[1 1 1] Check if we already have draw sphere in draw manager and if yes break loop...
                  (if (`KismetStringLibrary.EqualEqual_StrStr` (`KismetSystemLibrary.GetObjectName` _array_element) (`KismetSystemLibrary.GetObjectName` self))
                    (set `self.bHasSelfInManager` true)
                    (break)))
                ;;[1 1 1] ... and add self to draw manager
                (if (not (`self.bHasSelfInManager`))
                  (`KismetArrayLibrary.Array_Add` _drawingspheres self))))
            (:`CastFailed`
              (`KismetSystemLibrary.PrintString` "ERROR! Tag \"DrawManager\" is not on the draw manager!" true true (struct :`R` 1.0 :`A` 1.0) 5.0 "DrawSphere")))
          (else
            (`KismetSystemLibrary.PrintString` "ERROR! More than 1 DrawManager!" true true (struct :`R` 1.0 :`A` 1.0) 5.0 "DrawSphere")))))))